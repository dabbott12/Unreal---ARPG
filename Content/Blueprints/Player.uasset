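; Player character Blueprint for a melee game with movement, jumping, blocking and attacking.
; Blocking and Attacking flags gate movement, jumping and new attacks, with Attacking clearing after a fixed delay.
; Mouse X yaws the controller, while Mouse Y pitches the spring arm within clamped limits.
; TryDealDamage damages and logs Enemy actors overlapping DamageCollider, but nothing in these graphs calls it.
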(event Input|ActionEvents|InputActionJump
  (params (Key :type Key%20Structure :default "None"))
  ;[1 1 1] Inputs
  ;;[1 1 1] Jumping
  (:Pressed
    (if (AI|Components|NavMovement|IsMovingonGround (Variables|Character|GetCharacterMovement))
      (if (not (or (Variables|Default|GetAttacking) (Variables|Default|GetBlocking)))
        (Character|Jump)))))

(event Input|ActionEvents|InputActionAttack
  (params (Key :type Key%20Structure :default "None"))
  ;[1 1 1] Inputs
  ;;[1 1 1] Attacking
  (:Pressed
    (if (not (or (Variables|Default|GetAttacking) (Variables|Default|GetBlocking)))
      (Variables|Default|SetAttacking true)
      (Utilities|FlowControl|Delay 1.5)
      (Variables|Default|SetAttacking false))))

(event Input|ActionEvents|InputActionBlock
  (params (Key :type Key%20Structure :default "None"))
  ;[1 1 1] Inputs
  ;;[1 1 1] Blocking
  (:Pressed
    (if (not (Variables|Default|GetAttacking))
      (Variables|Default|SetBlocking true)))
  (:Released
    (Variables|Default|SetBlocking false)))

(event Input|AxisEvents|InputAxisMove_ForwardBack
  (params (AxisValue :type Float%20%28single-precision%29))
  ;[1 1 1] Inputs
  ;;[1 1 1] Move Forward Or Back
  (if (not (or (Variables|Default|GetAttacking) (Variables|Default|GetBlocking)))
    (Pawn|Input|AddMovementInput (Transformation|GetActorForwardVector) AxisValue false)))

(event Input|AxisEvents|InputAxisMove_LeftRight
  (params (AxisValue :type Float%20%28single-precision%29))
  ;[1 1 1] Inputs
  ;;[1 1 1] Move Left Or Right
  (if (not (or (Variables|Default|GetAttacking) (Variables|Default|GetBlocking)))
    (Pawn|Input|AddMovementInput (Transformation|GetActorRightVector) AxisValue false)))

(event Input|MouseEvents|MouseX
  (params (AxisValue :type Float%20%28single-precision%29))
  ;[1 1 1] Camera
  ;;[1 1 1] Rotates Player Left And Right
  (Pawn|Input|AddControllerYawInput AxisValue))

(event Input|MouseEvents|MouseY
  (params (AxisValue :type Float%20%28single-precision%29))
  ;[1 1 1] Camera
  ;;[1 1 1] Rotates Camera Up And Down
  (Transformation|AddLocalRotation (Variables|Default|GetSpringArm) (Math|Rotator|MakeRotator 0.0 AxisValue 0.0) false false)
  (Transformation|SetRelativeRotation (Variables|Default|GetSpringArm) (Math|Rotator|MakeRotator 0.0 (Math|Float|ClampAngle (.Pitch (Math|Rotator|BreakRotator (Class|SpringArmComponent|GetTargetRotation (Variables|Default|GetSpringArm)))) -45.0 2e+01) 0.0) false false))

(fn ConstructionScript)

(fn TryDealDamage
  (for _array_element (Collision|GetOverlappingActors (Variables|Default|GetDamageCollider) "/Game/Blueprints/Enemy.Enemy_C" :!class /Script/Engine.PrimitiveComponent)
    (bind _asenemy (Utilities|Casting|CastToEnemy _array_element))
    (Default|TakeDamage _asenemy (Variables|Default|GetDamage))
    (Development|PrintString "Hit enemy!")))